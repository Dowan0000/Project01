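; BP_DefaultPawn is a mouse-driven pawn for selecting BP_Cube actors and showing their info through UI.
; On BeginPlay it adds a WBP_SaveUI widget and enables the cursor with game-and-UI input.
; Left click traces from the deprojected mouse position, passes a hit cube to the save widget, and opens a fresh WBP_Cube widget fed its location and rotation.
; Right click closes that cube widget.
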(event EventBeginPlay
  (bind _returnvalue (Game|GetPlayerController 0))
  (bind _returnvalue_2 (UserInterface|CreateWidget "/Game/_Game/UI/WBP_SaveUI.WBP_SaveUI_C"))
  (bind _output_get (Variables|Default|SetSaveWidget _returnvalue_2))
  (UserInterface|Viewport|AddtoViewport _output_get 0)
  (Input|SetInputModeGameandUI _returnvalue 0 "DoNotLock" true)
  (Variables|/Script/Engine.PlayerController|SetbShowMouseCursor _returnvalue true))

(event Collision|EventActorBeginOverlap
  (params (OtherActor :type Actor%20Object%20Reference)))

(event EventTick
  (params (DeltaSeconds :type Float%20%28single-precision%29)))

(event Input|MouseEvents|LeftMouseButton
  (params (Key :type Key%20Structure :default "None"))
  (bind _returnvalue (Game|GetPlayerController 0))
  (bind (_worldlocation _worlddirection) (Game|Player|ConvertMouseLocationToWorldSpace _returnvalue))
  (:Pressed
    (bind _outhit (Collision|LineTraceForObjects _worldlocation (+ _worldlocation (* _worlddirection 2e+04)) (Utilities|Array|MakeArray "ObjectTypeQuery1" "ObjectTypeQuery2" "ObjectTypeQuery3" "ObjectTypeQuery4" "ObjectTypeQuery5" "ObjectTypeQuery6") false 0 "None"))
    (bind _asbp_cube (Utilities|Casting|CastToBP_Cube (.HitActor (Collision|BreakHitResult _outhit))))
    (Variables|/Game/_Game/UI/WBP_SaveUI.WBP_SaveUI_C|SetCurCubeRef (Variables|Default|GetSaveWidget) _asbp_cube)
    (Utilities|IsValid (Variables|Default|GetCubeWidget)
      (:Is%20Valid
        (Widget|RemovefromParent (Variables|Default|GetCubeWidget)))
      (:Is%20Not%20Valid
        _))
    (bind _returnvalue_2 (UserInterface|CreateWidget "/Game/_Game/UI/WBP_Cube.WBP_Cube_C"))
    (bind _output_get (Variables|Default|SetCubeWidget _returnvalue_2))
    (UserInterface|Viewport|AddtoViewport _output_get 0)
    (Utilities|FlowControl|Sequence
      (:then_0
        (Variables|/Game/_Game/UI/WBP_Cube.WBP_Cube_C|SetLocation _output_get (Transformation|GetActorLocation (.HitActor (Collision|BreakHitResult _outhit)))))
      (:then_1
        (Variables|/Game/_Game/UI/WBP_Cube.WBP_Cube_C|SetRotation _output_get (Transformation|GetActorRotation (.HitActor (Collision|BreakHitResult _outhit))))))))

(event Input|MouseEvents|RightMouseButton
  (params (Key :type Key%20Structure :default "None"))
  (:Pressed
    (Utilities|IsValid (Variables|Default|GetCubeWidget)
      (:Is%20Valid
        (Widget|RemovefromParent (Variables|Default|GetCubeWidget))
        (Variables|Default|SetCubeWidget 0)))))

(fn ConstructionScript)
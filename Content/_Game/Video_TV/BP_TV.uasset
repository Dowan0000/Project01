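; BP_TV is an in-world TV that plays a video from FileURL and toggles between play and pause.
; Each instance constructs its own MediaTexture in the construction script and its own MediaPlayer on BeginPlay, wired to the texture and MediaSound before opening the URL.
; TogglePlayer flip-flops Play and Pause, and on first play creates a dynamic M_TV material on the mesh to display the texture.
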(event Custom|TogglePlayer
  (bind _mediaplayer (Variables|Default|GetMediaPlayer))
  (Utilities|FlowControl|FlipFlop
    (:A
      (Development|PrintString "111111111111")
      (Media|MediaPlayer|Play _mediaplayer :!class /Script/MediaAssets.MediaPlayer)
      (Utilities|FlowControl|DoOnce false
        (:Completed
          (bind _returnvalue (Rendering|Material|CreateDynamicMaterialInstance (Variables|Default|GetStaticMesh) 0 "/Game/_Game/Video/M_TV.M_TV" "None" :!class /Script/Engine.PrimitiveComponent))
          (Rendering|Material|SetTextureParameterValue _returnvalue "MediaTexture" (Variables|Default|GetMediaTexture)))))
    (:B
      (Sequencer|Player|Pause _mediaplayer))))

(event EventBeginPlay
  (bind _returnvalue (Game|ConstructObjectfromClass "/Script/MediaAssets.MediaPlayer" self))
  (bind _output_get (Variables|Default|SetMediaPlayer _returnvalue))
  (Media|MediaSoundComponent|SetMediaPlayer (Variables|Default|GetMediaSound) _output_get)
  (Media|MediaSoundComponent|SetMediaPlayer (Variables|Default|GetMediaTexture) _output_get)
  (Class|MediaPlayer|OpenUrl _output_get (Variables|Default|GetFileURL)))

(fn ConstructionScript
  (bind _returnvalue (Game|ConstructObjectfromClass "/Script/MediaAssets.MediaTexture" self))
  (Variables|Default|SetMediaTexture _returnvalue))
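; BP_Object is an actor that implements a Focus interface to give visual feedback when a caller focuses or unfocuses it.
; Focus and Unfocus pass through only for a locally controlled Caller, so the purely visual change shows just on that client.
; HandleFocusChange toggles Render Custom Depth on either the given primitive component or, when not component-based, the root and all its descendant primitives.
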(event Custom|Set%20Render%20Custom%20Depth%20for%20All
  (params (Value :type Boolean))
  (bind _rootcomponent (Variables|Transformation|GetRootComponent))
  ;[1 1 1] Focus Interface. Since it's purely visual, Only allow the Clients owning the Caller to see these changes
  ;;[1 1 1] Gets all Primitives and turns on/off Render Custom Depth
  (bind _asprimitive_component (Utilities|Casting|CastToPrimitiveComponent _rootcomponent)
    (:then
      (Rendering|SetRenderCustomDepth _asprimitive_component Value))
    (:CastFailed
      _))
  (for _array_element (Components|GetChildrenComponents _rootcomponent true)
    (bind _asprimitive_component_2 (Utilities|Casting|CastToPrimitiveComponent _array_element))
    (Rendering|SetRenderCustomDepth _asprimitive_component_2 Value)))

(event Custom|Handle%20Focus%20Change
  (params (Component :type Scene%20Component%20Object%20Reference) (Is%20Focused :type Boolean) (Component%20Based :type Boolean))
  ;[1 1 1] Focus Interface. Since it's purely visual, Only allow the Clients owning the Caller to see these changes
  (bind _asprimitive_component (Utilities|Casting|CastToPrimitiveComponent Component))
  (if Component%20Based
    (Rendering|SetRenderCustomDepth _asprimitive_component Is%20Focused)
    (else
      (CallFunction|SetRenderCustomDepthforAll Is%20Focused))))

(event EventBeginPlay)

(event Collision|EventActorBeginOverlap
  (params (OtherActor :type Actor%20Object%20Reference)))

(event EventTick
  (params (DeltaSeconds :type Float%20%28single-precision%29)))

(event EventFocus
  (params (Caller :type Transformer%20Pawn%20Object%20Reference) (Component :type Scene%20Component%20Object%20Reference) (bComponentBased :type Boolean))
  ;[1 1 1] Focus Interface. Since it's purely visual, Only allow the Clients owning the Caller to see these changes
  (if (Pawn|IsLocallyControlled Caller)
    (CallFunction|HandleFocusChange Component true bComponentBased)))

(event EventUnfocus
  (params (Caller :type Transformer%20Pawn%20Object%20Reference) (Component :type Scene%20Component%20Object%20Reference) (bComponentBased :type Boolean))
  ;[1 1 1] Focus Interface. Since it's purely visual, Only allow the Clients owning the Caller to see these changes
  (if (Pawn|IsLocallyControlled Caller)
    (CallFunction|HandleFocusChange Component false bComponentBased)))

(fn ConstructionScript)